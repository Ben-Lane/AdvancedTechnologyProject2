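; BP_ItemInventory tracks the player's counts of Health, Sword and Shield items in an Inventory struct.
; IncrementItemCount switches on the item type to build a one-item struct, then adds it field by field to Inventory.
; It prints all three totals after each increment, and BeginPlay is empty.
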(event `self.ReceiveBeginPlay`)

(fn `IncrementItemCount`
  (params (ItemType :type "/Game/GAME_CONTENT/Maps/CaptureFlag/ENUM_ItemType Enum" :default "NewEnumerator0"))
  (locals (Addition :type "/Game/GAME_CONTENT/Player/Items/S_Inventory Structure"))
  (bind (_addition_health _addition_sword _addition_shield) (break `/Game/GAME_CONTENT/Player/Items/S_Inventory` (`local.Addition`)))
  (bind (_inventory_health _inventory_sword _inventory_shield) (break `/Game/GAME_CONTENT/Player/Items/S_Inventory` (`self.Inventory`)))
  (switch `/Game/GAME_CONTENT/Maps/CaptureFlag/ENUM_ItemType` ItemType
    (:`NewEnumerator0`
      (set `local.Addition` (make `/Game/GAME_CONTENT/Player/Items/S_Inventory` 1)))
    (:`NewEnumerator1`
      (set `local.Addition` (make `/Game/GAME_CONTENT/Player/Items/S_Inventory` 0 1)))
    (:`NewEnumerator2`
      (set `local.Addition` (make `/Game/GAME_CONTENT/Player/Items/S_Inventory` 0 0 1))))
  (bind _output_get (set `self.Inventory` (make `/Game/GAME_CONTENT/Player/Items/S_Inventory` (+ _addition_health _inventory_health) (+ _addition_sword _inventory_sword) (+ _addition_shield _inventory_shield))))
  (`KismetSystemLibrary.PrintString` (`KismetStringLibrary.Conv_IntToString` (break `/Game/GAME_CONTENT/Player/Items/S_Inventory` _output_get)))
  (`KismetSystemLibrary.PrintString` (`KismetStringLibrary.Conv_IntToString` (`.Sword_7_3DC5478D47DF460156B3AEA835499C63` (break `/Game/GAME_CONTENT/Player/Items/S_Inventory` _output_get))))
  (`KismetSystemLibrary.PrintString` (`KismetStringLibrary.Conv_IntToString` (`.Shield_8_A15569C8467018DD9D090B847DBF9A81` (break `/Game/GAME_CONTENT/Player/Items/S_Inventory` _output_get)))))