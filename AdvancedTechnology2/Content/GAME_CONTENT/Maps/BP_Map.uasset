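; BP_Map is the level's map actor, marking the playable area and holding data for mapping GPS coordinates.
; SafeZoneBounds overlaps update the player character's InMapBounds flag and toggle an out-of-bounds HUD widget.
; Construction caches the SafeZone location as map center, and BeginPlay derives a map-to-world scale from fixed literals.
; Mercator-style FlattenGPS and DeFlattenGPS helpers convert coordinates, though the event graph's flatten calls are disconnected.
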(event `self.SafeZoneBounds.OnComponentBeginOverlap`
  (params (OverlappedComponent :type "PrimitiveComponent Object Reference") (OtherActor :type "Actor Object Reference") (OtherComp :type "PrimitiveComponent Object Reference") (OtherBodyIndex :type Integer) (bFromSweep :type Boolean) (SweepResult :type "HitResult Structure (by ref)"))
  ;[0 0.1922 0.2196 1 26] USER HAS ENTERED THE MAP BOUNDS
  (bind _asbp_third_person_character (cast `/Game/ThirdPerson/Blueprints/BP_ThirdPersonCharacter` OtherActor))
  (set `/Game/ThirdPerson/Blueprints/BP_ThirdPersonCharacter.InMapBounds` true _asbp_third_person_character)
  (`Widget.SetVisibility` (`/Game/GAME_CONTENT/UI/WBP_GameplayHUD.WBP_MapInBounds` (`/Game/ThirdPerson/Blueprints/BP_ThirdPersonCharacter.PlayerHUD` _asbp_third_person_character)) "Hidden")
  (`KismetSystemLibrary.PrintString` "EnteredBounds - Inside of Map"))

(event `self.SafeZoneBounds.OnComponentEndOverlap`
  (params (OverlappedComponent :type "PrimitiveComponent Object Reference") (OtherActor :type "Actor Object Reference") (OtherComp :type "PrimitiveComponent Object Reference") (OtherBodyIndex :type Integer))
  ;[0 0.1922 0.2196 1 26] PLAYER HAS EXITED THE MAP BOUNDS
  (bind _asbp_third_person_character (cast `/Game/ThirdPerson/Blueprints/BP_ThirdPersonCharacter` OtherActor))
  (set `/Game/ThirdPerson/Blueprints/BP_ThirdPersonCharacter.InMapBounds` false _asbp_third_person_character)
  (`Widget.SetVisibility` (`/Game/GAME_CONTENT/UI/WBP_GameplayHUD.WBP_MapInBounds` (`/Game/ThirdPerson/Blueprints/BP_ThirdPersonCharacter.PlayerHUD` _asbp_third_person_character)) "Visible")
  (`KismetSystemLibrary.PrintString` "LeftBounds - Out of Map"))

(event `self.ReceiveBeginPlay`
  ;[1 1 1] FIND WORLD SCALE
  (set `self.MapToWorldScale` (/ 1240.0 70.39)))

(fn `DeFlattenGPS`
  (params (GPS :type "/Game/GAME_CONTENT/Maps/S_GPS_Location Structure"))
  (returns (NewGPS :type "/Game/GAME_CONTENT/Maps/S_GPS_Location Structure"))
  (return (make `/Game/GAME_CONTENT/Maps/S_GPS_Location` (* (/ GPS_Longitude_8_004329D64FC0250D4DC27EB03A410132 6378137) (/ 180 (`KismetMathLibrary.RadiansToDegrees` (`KismetMathLibrary.GetPI`)))) (* (* (`KismetMathLibrary.DegAtan` (`KismetMathLibrary.Exp` (/ GPS_Latitude_9_01CD1820467810808C29EFAB85D827DE 6378137))) (- 2 (/ (`KismetMathLibrary.RadiansToDegrees` (`KismetMathLibrary.GetPI`)) 2))) (/ 180 (`KismetMathLibrary.RadiansToDegrees` (`KismetMathLibrary.GetPI`)))))))

(fn `FlattenGPS`
  (params (WorldLoc :type "/Game/GAME_CONTENT/Maps/S_GPS_Location Structure"))
  (returns (FlattenGPS :type "/Game/GAME_CONTENT/Maps/S_GPS_Location Structure"))
  (return (make `/Game/GAME_CONTENT/Maps/S_GPS_Location` (* (* 6378137 WorldLoc_Longitude_8_004329D64FC0250D4DC27EB03A410132) (/ (`KismetMathLibrary.RadiansToDegrees` (`KismetMathLibrary.GetPI`)) 180.0)) (* 6378137 (`KismetMathLibrary.Log` (`KismetMathLibrary.DegTan` (+ (/ (`KismetMathLibrary.RadiansToDegrees` (`KismetMathLibrary.GetPI`)) 4.0) (* (/ (`KismetMathLibrary.RadiansToDegrees` (`KismetMathLibrary.GetPI`)) 360.0) WorldLoc_Latitude_9_01CD1820467810808C29EFAB85D827DE))) 10.0)))))

(fn `UserConstructionScript`
  ;[0 0 0] FIND PLAYABLE MAP CENTER
  (set `self.MapCenter` (`SceneComponent.K2_GetComponentLocation` (`self.SafeZone`))))