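; BP_GPS is a Blueprint that starts device GPS tracking through Unreal's location services and prints the results as debug text.
; On BeginPlay it initializes the service at best accuracy with periodic updates, then prints whether it started.
; On success it binds LocationChanged to the service's update event, which prints each new longitude and latitude without storing them.
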(event `self.ReceiveBeginPlay`
  (`LocationServices.GetLocationServicesImpl`)
  (`LocationServices.InitLocationServices` "LA_Best" 5.0)
  (bind _returnvalue (`LocationServices.StartLocationServices`))
  (if _returnvalue
    (`KismetSystemLibrary.PrintString` "GPS_ON")
    (bind _returnvalue_2 (`LocationServices.GetLocationServicesImpl`))
    (add `LocationServicesImpl.OnLocationChanged` _returnvalue_2 (delegate `LocationChanged`))
    (else
      (`KismetSystemLibrary.PrintString` "GPS_OFF"))))

(event `LocationChanged`
  (params (LocationData :type "LocationServicesData Structure"))
  (`KismetSystemLibrary.PrintString` (`KismetStringLibrary.Conv_DoubleToString` LocationData_Longitude))
  (`KismetSystemLibrary.PrintString` (`KismetStringLibrary.Conv_DoubleToString` LocationData_Latitude)))

(fn `UserConstructionScript`)