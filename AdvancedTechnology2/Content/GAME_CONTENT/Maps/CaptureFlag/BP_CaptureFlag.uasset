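; Capture-the-flag actor that stays hidden until the player discovers it, then can be claimed by touch.
; Overlapping FoundCollision reveals the pole and flag, plays a grow timeline and adds the meshes to the character's show-only renderer for front-layer drawing.
; Construction sets material and ownership from FlagStatus; touching an unowned flag runs Battle if its material is Lost, otherwise Defend.
; The flag material doubles as state, and both events mark it owned.
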(event `self.FoundCollision.OnComponentBeginOverlap`
  (params (OverlappedComponent :type "PrimitiveComponent Object Reference") (OtherActor :type "Actor Object Reference") (OtherComp :type "PrimitiveComponent Object Reference") (OtherBodyIndex :type Integer) (bFromSweep :type Boolean) (SweepResult :type "HitResult Structure (by ref)"))
  ;[0.3385 0.2897 0] DISCOVER FLAG - RUN ANIMATION - ADD TO FRONT LAYER VISUAL RENDER
  (if (not (`self.Discovered`))
    (bind _asbp_third_person_character (cast `/Game/ThirdPerson/Blueprints/BP_ThirdPersonCharacter` OtherActor))
    (bind _layeringcamera (`/Game/ThirdPerson/Blueprints/BP_ThirdPersonCharacter.AccessMeshRenderer` _asbp_third_person_character))
    (`self.AddToMeshRenderer` _layeringcamera)
    (`self.ToggleFlagVisual` true)
    (`self.GrowFlag`)
    (set `self.Discovered` true)))

(event `Battle`
  ;[0 0.4 0.4314] BATTLE MODE
  (`PrimitiveComponent.SetMaterial` (`self.Flag`) 0 "/Game/GAME_CONTENT/Maps/CaptureFlag/MAT_FlagHeld.MAT_FlagHeld")
  (set `self.FlagOwned` true))

(event `Defend`
  ;[0 0.4 0.4314] DEFEND MODE
  (`PrimitiveComponent.SetMaterial` (`self.Flag`) 0 "/Game/GAME_CONTENT/Maps/CaptureFlag/MAT_FlagNeutral.MAT_FlagNeutral")
  (set `self.FlagOwned` true))

(event `GrowFlag`
  ;[0.3385 0.2897 0] DISCOVER FLAG - RUN ANIMATION - ADD TO FRONT LAYER VISUAL RENDER
  (bind (_direction _size) (`Timeline|Growth` :!via `PlayFromStart`)
    (:`Update`
      (`SceneComponent.SetRelativeScale3D` (`self.VisualPivot`) (`KismetMathLibrary.Conv_DoubleToVector` _size)))))

(event `self.FlagCollision.OnComponentBeginOverlap`
  (params (OverlappedComponent :type "PrimitiveComponent Object Reference") (OtherActor :type "Actor Object Reference") (OtherComp :type "PrimitiveComponent Object Reference") (OtherBodyIndex :type Integer) (bFromSweep :type Boolean) (SweepResult :type "HitResult Structure (by ref)"))
  ;[0.3177 0.3161 0 1 20] WHEN PLAYER TOUCHES FLAG, INITIATE GIVEN EVENT
  (cast `/Game/ThirdPerson/Blueprints/BP_ThirdPersonCharacter` OtherActor)
  (if (not (`self.FlagOwned`))
    (bind _battle_ (`self.BattleFlag`))
    (if _battle_
      (`self.Battle`)
      (else
        (`self.Defend`)))))

(fn `AddToMeshRenderer`
  (params (Renderer :type "SceneCaptureComponent2D Object Reference"))
  (`SceneCaptureComponent.ShowOnlyComponent` Renderer (`self.Pole`))
  (`SceneCaptureComponent.ShowOnlyComponent` Renderer (`self.PoleStand`))
  (`SceneCaptureComponent.ShowOnlyComponent` Renderer (`self.Base`))
  (`SceneCaptureComponent.ShowOnlyComponent` Renderer (`self.PoleTop`))
  (`SceneCaptureComponent.ShowOnlyComponent` Renderer (`self.Flag`)))

(fn `BattleFlag`
  (returns (`Battle?` :type Boolean))
  ;[0 1 0.915 1 58] CHECK STATE OF FLAG
  (return (== (`PrimitiveComponent.GetMaterial` (`self.Flag`) 0) "/Game/GAME_CONTENT/Maps/CaptureFlag/MAT_FlagLost.MAT_FlagLost")))

(fn `ToggleFlagVisual`
  (params (FlagCanBeSeen :type Boolean))
  (bind _pole (`self.Pole`))
  (bind _polestand (`self.PoleStand`))
  (bind _poletop (`self.PoleTop`))
  (bind _flag (`self.Flag`))
  ;[1 0 0 1 66] UPDATE FLAG POLE VISUAL ONLY
  (if FlagCanBeSeen
    (`SceneComponent.SetVisibility` _pole true false)
    (`SceneComponent.SetVisibility` _polestand true false)
    (`SceneComponent.SetVisibility` _poletop true false)
    (`SceneComponent.SetVisibility` _flag true false)
    (else
      (`SceneComponent.SetVisibility` _pole false false)
      (`SceneComponent.SetVisibility` _polestand false false)
      (`SceneComponent.SetVisibility` _poletop false false)
      (`SceneComponent.SetVisibility` _flag false false))))

(fn `UserConstructionScript`
  (`self.ToggleFlagVisual` false)
  ;[0.7664 1 0 1 50] SETUP DEFAULT FLAG COLOUR
  (switch `/Game/GAME_CONTENT/Maps/CaptureFlag/ENUM_FlagStatus` (`self.FlagStatus`)
    (:`NewEnumerator0`
      (`PrimitiveComponent.SetMaterial` (`self.Flag`) 0 "/Game/GAME_CONTENT/Maps/CaptureFlag/MAT_FlagHeld.MAT_FlagHeld")
      (set `self.FlagOwned` true))
    (:`NewEnumerator1`
      (`PrimitiveComponent.SetMaterial` (`self.Flag`) 0 "/Game/GAME_CONTENT/Maps/CaptureFlag/MAT_FlagNeutral.MAT_FlagNeutral")
      (set `self.FlagOwned` false))
    (:`NewEnumerator2`
      (`PrimitiveComponent.SetMaterial` (`self.Flag`) 0 "/Game/GAME_CONTENT/Maps/CaptureFlag/MAT_FlagLost.MAT_FlagLost")
      (set `self.FlagOwned` false))))