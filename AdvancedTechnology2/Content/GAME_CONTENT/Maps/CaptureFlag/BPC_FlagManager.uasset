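; Capture-flag manager component on BP_Map that spawns flags at random map spawn points and tracks their discovery.
; At BeginPlay it caps the count to available FlagSpawns children, spawns flags named after their points, and destroys used points to prevent repeats.
; Flag event dispatchers update the player HUD by list index: discovery updates name entries and creates info tabs, and overlap end animates the matching tab.
; GenerateFlagType, an even type-distribution helper, is uncalled here.
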(event `ED_EndFlagOverlap`
  (params (FlagRef :type "/Game/GAME_CONTENT/Maps/CaptureFlag/BP_CaptureFlag Object Reference"))
  ;[1 0.3434 0.8007 1 34] SETUP FLAG DISCOVERY INCREMENTATION
  (for _array_element (`PanelWidget.GetAllChildren` (`/Game/GAME_CONTENT/UI/WBP_GameplayHUD.InfoTabs` (`/Game/ThirdPerson/Blueprints/BP_ThirdPersonCharacter.PlayerHUD` (`self.PlayerRef`))))
    (bind _aswbp_informationbutton (cast `/Game/GAME_CONTENT/UI/WBP_Informationbutton` _array_element))
    (if (== (`/Game/GAME_CONTENT/UI/WBP_Informationbutton.LocationIndex` _aswbp_informationbutton) (`KismetArrayLibrary.Array_Find` (`self.FlagList`) FlagRef))
      (`/Game/GAME_CONTENT/UI/WBP_Informationbutton.TabAnimation` _aswbp_informationbutton false)
      (break))))

(event `self.ReceiveBeginPlay`
  (bind _children (`SceneComponent.GetChildrenComponents` (`/Game/GAME_CONTENT/Maps/BP_Map.FlagSpawns` (`self.OwnerMap`)) false))
  (bind _returnvalue (`KismetArrayLibrary.Array_Length` (`SceneComponent.GetChildrenComponents` (`/Game/GAME_CONTENT/Maps/BP_Map.FlagSpawns` (`self.OwnerMap`)) false)))
  ;[1 1 1 1 58] INITIATE FLAGS - SPAWN 6 RANDOM FROm BP_MAP LAYOUT
  (bind _asbp_third_person_character (cast `/Game/ThirdPerson/Blueprints/BP_ThirdPersonCharacter` (`GameplayStatics.GetPlayerCharacter` 0)))
  (set `self.PlayerRef` _asbp_third_person_character)
  (`KismetArrayLibrary.Array_Clear` (`self.FlagList`))
  (bind _asbp_map (cast `/Game/GAME_CONTENT/Maps/BP_Map` (`self.GetOwner`)))
  (set `self.OwnerMap` _asbp_map)
  (if (> (`self.FlagsToSpawn`) _returnvalue)
    (set `self.FlagsToSpawn` _returnvalue))
  (while (not (`self.SpawnedAllFlags`))
    (if (> (`self.FlagsToSpawn`) 0)
      (`self.SpawnFlag` (`|GetArrayItem` _children (`KismetMathLibrary.RandomIntegerInRange` 0 (- (`KismetArrayLibrary.Array_Length` _children) 1))))
      ;[1 0.3434 0.8007 1 34] SETUP FLAG DISCOVERY INCREMENTATION
      (for _array_element (`self.FlagList`)
        (add `/Game/GAME_CONTENT/Maps/CaptureFlag/BP_CaptureFlag.ED_FlagDiscovered` _array_element (delegate `ED_FlagDiscovered_Event`))
        (add `/Game/GAME_CONTENT/Maps/CaptureFlag/BP_CaptureFlag.ED_EndFlagOverlap` _array_element (delegate `ED_EndFlagOverlap`)))
      (else
        (set `self.SpawnedAllFlags` true)))))

(event `ED_FlagDiscovered_Event`
  (params (FlagRef :type "/Game/GAME_CONTENT/Maps/CaptureFlag/BP_CaptureFlag Object Reference"))
  (bind _returnvalue (`KismetArrayLibrary.Array_Find` (`self.FlagList`) FlagRef))
  (bind _playerhud (`/Game/ThirdPerson/Blueprints/BP_ThirdPersonCharacter.PlayerHUD` (`self.PlayerRef`)))
  (bind _returnvalue_2 (`PanelWidget.GetChildAt` (`/Game/GAME_CONTENT/UI/WBP_GameplayHUD.FlagNameList` _playerhud) _returnvalue))
  ;[1 0.3434 0.8007 1 34] SETUP FLAG DISCOVERY INCREMENTATION
  (set `self.FlagsFound` (+ (`self.FlagsFound`) 1))
  (if (and (`KismetSystemLibrary.DoesImplementInterface` _returnvalue_2 "/Game/GAME_CONTENT/Maps/CaptureFlag/BPI_FlagTracking.BPI_FlagTracking_C") (== _returnvalue (`/Game/GAME_CONTENT/UI/WBP_GameplayHUD.TrackedFlag` _playerhud)))
    (message `/Game/GAME_CONTENT/Maps/CaptureFlag/BPI_FlagTracking.UnTrackFlag` _returnvalue_2)
    (else
      (message `/Game/GAME_CONTENT/Maps/CaptureFlag/BPI_FlagTracking.FoundFlag` _returnvalue_2)))
  (`/Game/GAME_CONTENT/UI/WBP_GameplayHUD.CreateInfoTab` (`/Game/ThirdPerson/Blueprints/BP_ThirdPersonCharacter.PlayerHUD` (`self.PlayerRef`)) (`/Game/GAME_CONTENT/Maps/CaptureFlag/BP_CaptureFlag.FlagName` FlagRef) _returnvalue)
  (`KismetSystemLibrary.PrintString` "New Info Tab"))

(fn `GenerateFlagType`
  (params (Index :type Integer))
  (locals (TypeOfFlag :type Integer))
  ;[1 1 1] DISTRIBUTES FLAG TYPES EVENLY BETWEEN TOTAL FLAGS TO BE SPAWNED
  (for _index (range (enumcount `/Game/GAME_CONTENT/Maps/CaptureFlag/ENUM_ItemType`))
    (if (< (`KismetMathLibrary.Conv_IntToDouble` Index) (* (/ (+ (`KismetArrayLibrary.Array_Length` (`self.FlagList`)) (`self.FlagsToSpawn`)) (enumcount `/Game/GAME_CONTENT/Maps/CaptureFlag/ENUM_ItemType`)) (+ _index 1)))
      (set `local.TypeOfFlag` _index)
      (break))))

(fn `SpawnFlag`
  (params (SpawnPoint :type "SceneComponent Object Reference"))
  ;[0.2618 1 0.027 1 50] CREATE FLAG AT SPAWN POINT - REMOVE FROM LIST OF FUTURE SPAWN POINTS
  (bind _returnvalue (`|SpawnActorFromClass` "/Game/GAME_CONTENT/Maps/CaptureFlag/BP_CaptureFlag.BP_CaptureFlag_C" (`KismetMathLibrary.MakeTransform` (`SceneComponent.K2_GetComponentLocation` SpawnPoint)) "Undefined" "MultiplyWithRoot" null "NewEnumerator2" (`KismetSystemLibrary.GetObjectName` SpawnPoint) (`self.PlayerRef`) null))
  (`/Game/GAME_CONTENT/Maps/CaptureFlag/BP_CaptureFlag.UpdateFlagText` _returnvalue)
  (`KismetArrayLibrary.Array_Add` (`self.FlagList`) _returnvalue)
  (set `self.FlagsToSpawn` (- (`self.FlagsToSpawn`) 1))
  (`SceneComponent.K2_DetachFromComponent` SpawnPoint "KeepRelative" "KeepRelative" "KeepRelative" true)
  (`self.K2_DestroyComponent` SpawnPoint))