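; Actor component that drives fog of war by painting its owner's position and explored area into render targets.
; On BeginPlay it creates dynamic instances of the fog render and reveal materials and sets their reveal size.
; Each tick a vertical complex trace through the owner finds the fog plane's collision UV.
; That UV becomes both materials' Location, and each is drawn into its own render target.
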(event `self.ReceiveBeginPlay`
  ;[0 0 0] SETUP FOG MATERIAL INSTANCES
  (bind _returnvalue (`KismetMaterialLibrary.CreateDynamicMaterialInstance` "/Game/GAME_CONTENT/Maps/Fog-of-War/MAT_FogRender.MAT_FogRender"))
  (set `self.FogRenderMaterial` _returnvalue)
  (bind _returnvalue_2 (`KismetMaterialLibrary.CreateDynamicMaterialInstance` "/Game/GAME_CONTENT/Maps/Fog-of-War/MAT_FogReveal.MAT_FogReveal"))
  (set `self.FogRevealMaterial` _returnvalue_2)
  ;[0 0 0] SET RENDER + REVEAL RANGE
  (`MaterialInstanceDynamic.SetScalarParameterValue` (`self.FogRenderMaterial`) "Size" (`self.FogRevealSize`))
  (`MaterialInstanceDynamic.SetScalarParameterValue` (`self.FogRevealMaterial`) "Size" (`self.FogRevealSize`)))

(event `self.ReceiveTick`
  (params (DeltaSeconds :type "Float (single-precision)"))
  (bind _returnvalue (`Actor.K2_GetActorLocation` (`self.GetOwner`)))
  ;[0.0302 0.3125 0] FIND PLAYER POSITION IN FOG PLANE - CONVERTS POSITION TO POSITION IN RENDER TARGET - ADDS EXPLORATION TO RENDER TARGET
  (bind _outhit (`KismetSystemLibrary.LineTraceSingle` (+ _returnvalue (0.0 0.0 500.0)) (+ _returnvalue (0.0 0.0 -500.0)) "TraceTypeQuery3" true))
  (bind _uv (`GameplayStatics.FindCollisionUV` _outhit))
  (`MaterialInstanceDynamic.SetVectorParameterValue` (`self.FogRenderMaterial`) "Location" (make `LinearColor` (`KismetMathLibrary.BreakVector2D` _uv) (`.Y` (`KismetMathLibrary.BreakVector2D` _uv)) 0.0 1.0))
  (`MaterialInstanceDynamic.SetVectorParameterValue` (`self.FogRevealMaterial`) "Location" (make `LinearColor` (`KismetMathLibrary.BreakVector2D` _uv) (`.Y` (`KismetMathLibrary.BreakVector2D` _uv)) 0.0 1.0))
  (`KismetRenderingLibrary.DrawMaterialToRenderTarget` "/Game/GAME_CONTENT/Maps/Fog-of-War/RT_FogRender.RT_FogRender" (`self.FogRenderMaterial`))
  (`KismetRenderingLibrary.DrawMaterialToRenderTarget` "/Game/GAME_CONTENT/Maps/Fog-of-War/RT_FogReveal.RT_FogReveal" (`self.FogRevealMaterial`)))